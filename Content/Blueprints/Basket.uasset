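; Player-controlled basket actor for an apple-catching game, with stacked basket meshes that act as lives.
; BeginPlay adds the TreeControls Enhanced Input context, binds to PickerState's apple-dropped event and caches the child static meshes in an array.
; MoveRight input slides the actor along its local Y axis, scaled by Speed and delta time.
; ReceiveDamage lowers Health and destroys a basket mesh, or opens MainScene when none remain to spare.
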(event Input|EnhancedActionEvents|EnhancedInputActionMoveRight
  (params (ActionValue :type Vector%202D%20Structure) (ElapsedSeconds :type Float%20%28double-precision%29) (TriggeredSeconds :type Float%20%28double-precision%29) (InputAction :type Input%20Action%20Object%20Reference :default "/Game/Bindings/MoveRight.MoveRight"))
  (CallFunction|Move (stale EventTick DeltaSeconds) (* (.x ActionValue) (Variables|Default|Getspeed))))

(event EventBeginPlay
  (bind _asplayer_controller (Utilities|Casting|CastToPlayerController (Game|GetPlayerController 0)))
  (Utilities|IsValid (PlayerController|LocalPlayerSubsystems|GetEnhancedInputLocalPlayerSubsystem _asplayer_controller)
    (:Is%20Valid
      (Input|AddMappingContext (PlayerController|LocalPlayerSubsystems|GetEnhancedInputLocalPlayerSubsystem _asplayer_controller) "/Game/Bindings/TreeControls.TreeControls" 0 "(bIgnoreAllPressedKeysUntilRelease=True,bForceImmediately=False,bNotifyUserSettings=False)")
      (bind _aspicker_state (Utilities|Casting|CastToPickerState (Game|GetGameState)))
      (bind _output_get (Variables|Default|SetPickerState _aspicker_state))
      (EventDispatchers|BindEventtoOnAppleDropped _output_get (EventDispatchers|CreateEvent :!event ReceiveDamage))
      (for _array_element (Components|GetChildrenComponents (Variables|Default|GetDefaultSceneRoot) false)
        (bind _asstatic_mesh_component (Utilities|Casting|CastToStaticMeshComponent _array_element))
        (Utilities|Array|Add (Variables|Default|GetBasketArray) _asstatic_mesh_component)))))

(event Collision|EventActorBeginOverlap
  (params (OtherActor :type Actor%20Object%20Reference)))

(event EventTick
  (params (DeltaSeconds :type Float%20%28single-precision%29)))

(fn ConstructionScript)

(fn Move
  (params (DeltaTime :type Float%20%28double-precision%29) (Speed :type Float%20%28double-precision%29))
  (Transformation|AddActorLocalOffset (Math|Vector|MakeVector 0.0 (* Speed DeltaTime) 0.0) false false))

(fn ReceiveDamage
  (if (> (Variables|Default|GetHealth) 1)
    (bind _result (Math|Integer|DecrementInt (Variables|Default|GetHealth))
      (:%20%20
        (Components|DestroyComponent (Utilities|Array|Get(acopy) (Variables|Default|GetBasketArray) _result))))
    (else
      (Game|OpenLevel(byObjectReference) "/Game/MainScene.MainScene"))))

(fn TryDeleteBasket)