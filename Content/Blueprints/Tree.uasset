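; Tree is an actor that slides back and forth along X while randomly dropping apples, as in an Apple Picker-style game.
; Each tick it flips the sign of Speed whenever its X location is outside the symmetric edge limits, then applies a frame-rate-scaled local offset without sweep.
; A looping timer rolls against ChanceToDropApple and, on success, spawns an Apple at one of two randomly chosen spawn points.
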(event EventBeginPlay
  (Utilities|Time|SetTimerbyFunctionName 0 "TryDropApple" 1.0 true))

(event Collision|EventActorBeginOverlap
  (params (OtherActor :type Actor%20Object%20Reference)))

(event EventTick
  (params (DeltaSeconds :type Float%20%28single-precision%29))
  (CallFunction|TryChangeDirection)
  (CallFunction|Move DeltaSeconds))

(fn ConstructionScript)

(fn TryDropApple
  (if (>= (Math|Random|RandomInteger 100) (- 100 (Variables|Default|GetchanceToDropApple)))
    (if (> (Math|Random|RandomInteger 2) 0)
      (Game|SpawnActorfromClass "/Game/Blueprints/Apple.Apple_C" (Transformation|GetWorldTransform (Variables|Default|GetSpawnPoint1)) "Undefined" "MultiplyWithRoot" 0 0)
      (else
        (Game|SpawnActorfromClass "/Game/Blueprints/Apple.Apple_C" (Transformation|GetWorldTransform (Variables|Default|GetSpawnPoint2)) "Undefined" "MultiplyWithRoot" 0 0)))))

(fn TryChangeDirection
  (bind _returnvalue (Transformation|GetActorLocation))
  (bind _leftandrightedge (Variables|Default|GetleftAndRightEdge))
  (bind _x (Math|Vector|BreakVector _returnvalue))
  (if (>= _x (* _leftandrightedge -1.0))
    (if (not (<= _x _leftandrightedge))
      (CallFunction|ChangeDirection :!label _label))
    (else
      (goto _label))))

(fn ChangeDirection
  (Variables|Default|Setspeed (* (Variables|Default|Getspeed) -1.0)))

(fn Move
  (params (DeltaTime :type Float%20%28double-precision%29))
  (Transformation|AddActorLocalOffset (Math|Vector|MakeVector (* (Variables|Default|Getspeed) DeltaTime) 0.0 0.0) false false))